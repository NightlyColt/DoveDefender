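; Test actor Blueprint that exercises function and delegate types exposed by its parent class.
; On BeginPlay it calls a callable function, a native event and a pure function whose result is printed, then binds two events to the OnDefault delegate.
; The native event override calls the parent version before printing its own message.
; The custom events AAA and BBB print their parameter's display name, BBB with a suffix.
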(event `self.ReceiveBeginPlay`
  (`self.BlueprintCallable`)
  (`self.BlueprintNativeEvent`)
  (`KismetSystemLibrary.PrintString` (`KismetStringLibrary.Conv_DoubleToString` (`self.Pure`)))
  (add `self.OnDefault` (`|CreateDelegate` :!event `AAA`))
  (add `self.OnDefault` (`|CreateDelegate` :!event `BBB`)))

(event `self.BlueprintNativeEvent`
  (`parent.BlueprintNativeEvent`)
  (`KismetSystemLibrary.PrintString` "In Blueprint"))

(event `AAA` :!signature `self.OnDefault`
  (params (NewParam :type "Actor Object Reference"))
  (`KismetSystemLibrary.PrintString` (`KismetSystemLibrary.GetDisplayName` NewParam)))

(event `BBB` :!signature `self.OnDefault`
  (params (NewParam :type "Actor Object Reference"))
  (`KismetSystemLibrary.PrintString` (`KismetStringLibrary.Concat_StrStr` (`KismetSystemLibrary.GetDisplayName` NewParam) "bbb")))

(fn `UserConstructionScript`)