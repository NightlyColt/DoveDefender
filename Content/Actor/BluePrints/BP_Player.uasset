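; BP_Player is the player-controlled character, handling look, movement and shooting input.
; On BeginPlay it runs the parent logic, adds a WBP_HUD widget to the viewport and binds to BPHealthComponent's damage and death events, or prints a warning without a PlayerController.
; Movement follows control yaw only, so camera pitch does not affect direction.
; The Shoot action calls CharacterShoot.
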(event `self.ReceiveBeginPlay`
  (`parent.ReceiveBeginPlay`)
  (bind _asplayer_controller (cast `PlayerController` (`self.GetController`))
    (:`then`
      (bind _returnvalue (`|CreateWidget` "/Game/Core/Widgets/WBP_HUD.WBP_HUD_C" _asplayer_controller))
      (bind _output_get (set `self.HUD` _returnvalue))
      (`UserWidget.AddToViewport` _output_get 0)
      (add `/Game/Core/Components/BP_Health_Component.OnDamaged` (`self.BP_Health_Component`) (`|CreateDelegate` (`self.HUD`) :!event `SetHealth`))
      (add `/Game/Core/Components/BP_Health_Component.OnDeath` (`self.BP_Health_Component`) (`|CreateDelegate` (`self.HUD`) :!event `SetHealth`)))
    (:`CastFailed`
      (`KismetSystemLibrary.PrintString` "Need Player for HUD"))))

(event `InputAxis|TurnTo`
  (params (AxisValue :type "Float (single-precision)"))
  ;[1 1 1] Rotation
  (`self.AddControllerYawInput` AxisValue))

(event `InputAxis|LookUp`
  (params (AxisValue :type "Float (single-precision)"))
  ;[1 1 1] Rotation
  (`self.AddControllerPitchInput` AxisValue))

(event `InputAxis|MoveForward`
  (params (AxisValue :type "Float (single-precision)"))
  (bind (_returnvalue_roll _returnvalue_pitch _returnvalue_yaw) (`KismetMathLibrary.BreakRotator` (`self.GetControlRotation`)))
  (`self.AddMovementInput` (`KismetMathLibrary.GetForwardVector` (`KismetMathLibrary.MakeRotator` 0.0 0.0 _returnvalue_yaw)) AxisValue))

(event `InputAxis|MoveSideways`
  (params (AxisValue :type "Float (single-precision)"))
  (bind (_returnvalue_roll _returnvalue_pitch _returnvalue_yaw) (`KismetMathLibrary.BreakRotator` (`self.GetControlRotation`)))
  (`self.AddMovementInput` (`KismetMathLibrary.GetRightVector` (`KismetMathLibrary.MakeRotator` 0.0 0.0 _returnvalue_yaw)) AxisValue))

(event `InputAction|Shoot`
  (params (Key :type "Key Structure"))
  (:`Pressed`
    (`self.CharacterShoot`)))

(fn `UserConstructionScript`
  (`parent.UserConstructionScript`))