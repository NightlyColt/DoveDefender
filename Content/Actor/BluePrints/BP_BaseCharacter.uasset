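; BP_BaseCharacter is a base character Blueprint that equips a weapon and forwards shooting to it.
; On BeginPlay it spawns the configured weapon class through a child actor component and caches it as a BP_BaseWeapon.
; It caches the mesh's ABP_Rifle anim instance and binds to the weapon's shoot and animation's action-complete events, printing errors if either cast fails.
; CharacterShoot calls Shoot on the current weapon.
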(event `self.ReceiveBeginPlay`
  (bind _weaponchild (`self.WeaponChild`))
  (`ChildActorComponent.SetChildActorClass` _weaponchild (`self.WeaponClass`))
  (bind _asbp_base_weapon (cast `/Game/Actor/BluePrints/BP_BaseWeapon` (`ChildActorComponent.ChildActor` _weaponchild))
    (:`then`
      (set `self.CurrentWeapon` _asbp_base_weapon)
      (bind _asabp_rifle (cast `/Game/Core/ABP_Rifle` (`SkeletalMeshComponent.GetAnimInstance` (`self.Mesh`)))
        (:`then`
          (set `self.AnimBP` _asabp_rifle)
          (add `/Game/Actor/BluePrints/BP_BaseWeapon.OnShoot` (`self.CurrentWeapon`) (`|CreateDelegate` (`self.AnimBP`) :!event `PlayShootAnim`))
          (add `/Game/Core/ABP_Rifle.OnActionComplete` (`self.AnimBP`) (`|CreateDelegate` (`self.CurrentWeapon`) :!event `StopAnimation`)))
        (:`CastFailed`
          (`KismetSystemLibrary.PrintString` "Animation Class unvalid"))))
    (:`CastFailed`
      (`KismetSystemLibrary.PrintString` "There's no weapon to use"))))

(event `CharacterShoot`
  (`/Game/Actor/BluePrints/BP_BaseWeapon.Shoot` (`self.CurrentWeapon`)))

(fn `UserConstructionScript`)