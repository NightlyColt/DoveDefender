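; Base weapon actor that fires projectiles for the pawn it is attached to as a child actor.
; On BeginPlay it caches the parent pawn as owner, printing a warning if none exists.
; Shoot spawns the projectile class at the muzzle socket along the pawn's aim rotation and calls the OnShoot dispatcher.
; A DoShoot flag blocks further shots until StopAnimation clears it.
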(event `self.ReceiveBeginPlay`
  (bind _aspawn (cast `Pawn` (`self.GetParentActor`))
    (:`then`
      (set `self.OwningPawn` _aspawn))
    (:`CastFailed`
      (`KismetSystemLibrary.PrintString` "We need a pawn to own this weapon"))))

(event `Shoot`
  (bind _owningpawn (`self.OwningPawn`))
  (if (`self.CanShoot`)
    (`|SpawnActorFromClass` (`self.ProjectileClass`) (`KismetMathLibrary.MakeTransform` (`SceneComponent.GetSocketLocation` (`self.SkeletalMesh`) "MuzzleFlashSocket") (`Pawn.GetBaseAimRotation` _owningpawn)) "Undefined" "OverrideRootScale" (`Pawn.GetController` _owningpawn) _owningpawn)
    (set `self.Do Shoot` true)
    (`self.OnShoot`)))

(event `StopAnimation`
  (set `self.Do Shoot` false))

(fn `CanShoot`
  (returns (DoShoot :type Boolean))
  (return (not (`self.Do Shoot`))))

(fn `UserConstructionScript`)