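; Base character Blueprint that links a weapon, a health component and the rifle animation Blueprint for shooting, damage and death.
; On BeginPlay it spawns the weapon class through a child actor component, caches it and the anim instance, then binds their event dispatchers.
; Damage plays a hit animation, while death stops movement, plays the death animation, disables capsule collision and flags the weapon dead.
; CharacterShoot forwards to the weapon, and CharacterDeathFinished is left empty.
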(event `self.ReceiveBeginPlay`
  (bind _weaponchild (`self.WeaponChild`))
  ;[1 1 1] Coded
  (`ChildActorComponent.SetChildActorClass` _weaponchild (`self.WeaponClass`))
  (bind _asbp_base_weapon (cast `/Game/BlueprintsVersion/Actor/BluePrints/BP_BaseWeapon` (`ChildActorComponent.ChildActor` _weaponchild))
    (:`then`
      (set `self.CurrentWeapon` _asbp_base_weapon)
      (bind _asabp_rifle (cast `/Game/Core/ABP_Rifle` (`SkeletalMeshComponent.GetAnimInstance` (`self.Mesh`)))
        (:`then`
          (set `self.AnimBP` _asabp_rifle)
          (add `/Game/BlueprintsVersion/Actor/BluePrints/BP_BaseWeapon.OnShoot` (`self.CurrentWeapon`) (`|CreateDelegate` (`self.AnimBP`) :!event `PlayShootAnim`))
          (add `RifleAnim.OnActionCompleteD` (`self.AnimBP`) (`|CreateDelegate` (`self.CurrentWeapon`) :!event `StopAnimation`))
          (add `HealthComponent.OnDeath` (`self.BP_Health_Component`) (`|CreateDelegate` :!event `CharacterDeath`))
          (add `HealthComponent.OnDamaged` (`self.BP_Health_Component`) (`|CreateDelegate` :!event `CharacterDamaged`))
          (add `/Game/Core/ABP_Rifle.OnDeathFinished` (`self.AnimBP`) (`|CreateDelegate` :!event `CharacterDeathFinished`)))
        (:`CastFailed`
          (`KismetSystemLibrary.PrintString` "Animation Class unvalid"))))
    (:`CastFailed`
      (`KismetSystemLibrary.PrintString` "There's no weapon to use"))))

(event `CharacterDeathFinished`)

(event `CharacterDeath`
  (params (Ratio :type "Float (double-precision)"))
  ;[1 1 1] Coded
  (`MovementComponent.StopMovementImmediately` (`self.CharacterMovement`))
  (`RifleAnim.PlayDeathAnim` (`self.AnimBP`) 0.0)
  (`PrimitiveComponent.SetCollisionEnabled` (`self.CapsuleComponent`) "NoCollision")
  (set `/Game/BlueprintsVersion/Actor/BluePrints/BP_BaseWeapon.Dead` true (`self.CurrentWeapon`)))

(event `CharacterDamaged`
  (params (Ratio :type "Float (double-precision)"))
  ;[1 1 1] Coded
  (`RifleAnim.PlayHitAnim` (`self.AnimBP`)))

(event `CharacterShoot`
  ;[1 1 1] Coded
  (`/Game/BlueprintsVersion/Actor/BluePrints/BP_BaseWeapon.Shoot` (`self.CurrentWeapon`)))

(fn `UserConstructionScript`)