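; BP_BaseAI is a base AI-controlled character that can shoot and die, building on its parent character's behavior.
; A Shoot event forwards to CharacterShoot.
; On death it runs the parent logic, then stops the AI controller's brain component so decision-making ends.
; When death finishes, it calls the parent handler and destroys the actor.
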(event `/Game/Interfaces/BPI_Weapon.Shoot`
  (`self.CharacterShoot`))

(event `self.CharacterDeathFinished`
  (`parent.CharacterDeathFinished`)
  (`self.K2_DestroyActor`))

(event `self.CharacterDeath`
  (params (Ratio :type "Float (single-precision)"))
  (`parent.CharacterDeath` Ratio)
  (`BrainComponent.StopLogic` (`AIController.BrainComponent` (`AIBlueprintHelperLibrary.GetAIController` self)) "AI is Dead"))

(fn `UserConstructionScript`
  (`parent.UserConstructionScript`))