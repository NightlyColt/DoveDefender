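; Base weapon actor that fires projectiles for its parent actor, which it expects to be a Pawn.
; Shoot spawns the projectile at the muzzle socket along the pawn's base aim rotation, then broadcasts OnShoot.
; DoShoot blocks further shots until StopAnimation clears it, as does the Dead flag.
; GetShotRotation, an alternative aim using the HUD's aimed point with an AI fallback, is unused.
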(event `self.ReceiveBeginPlay`
  ;[1 1 1] Coded
  (bind _aspawn (cast `Pawn` (`self.GetParentActor`))
    (:`then`
      (set `self.OwningPawn` _aspawn))
    (:`CastFailed`
      (`KismetSystemLibrary.PrintString` "We need a pawn to own this weapon"))))

(event `Shoot`
  (bind _owningpawn (`self.OwningPawn`))
  ;[1 1 1] Coded
  (if (`self.CanShoot`)
    (`|SpawnActorFromClass` (`self.ProjectileClass`) (`KismetMathLibrary.MakeTransform` (`SceneComponent.GetSocketLocation` (`self.SkeletalMesh`) "MuzzleFlashSocket") (`Pawn.GetBaseAimRotation` _owningpawn)) "Undefined" "OverrideRootScale" (`Pawn.GetController` _owningpawn) _owningpawn)
    (set `self.Do Shoot` true)
    (`self.OnShoot`)))

(event `StopAnimation`
  ;[1 1 1] Coded
  (set `self.Do Shoot` false))

(fn `CanShoot`
  (returns (DoShoot :type Boolean))
  ;[1 1 1] Coded
  (return (and (not (`self.Do Shoot`)) (not (`self.Dead`)))))

(fn `GetShotRotation`
  (returns (Rotation :type "Rotator Structure"))
  (locals (Destination :type "Vector Structure"))
  (bind _foundwidgets (`WidgetBlueprintLibrary.GetAllWidgetsOfClass` "/Game/Core/Widgets/WBP_HUD.WBP_HUD_C"))
  (bind _output (`|GetArrayItem` _foundwidgets))
  (if (== (`UserWidget.GetOwningPlayerPawn` _output) (`self.OwningPawn`))
    (bind (_valid _hitlocation _endpoint) (`/Game/Core/Widgets/WBP_HUD.GetAimedPoint` _output))
    (if _valid
      (set `local.Destination` _hitlocation)
      (else
        (set `local.Destination` _endpoint)))
    (return (`KismetMathLibrary.MakeRotFromX` (- (`local.Destination`) (`SceneComponent.GetSocketLocation` (`self.SkeletalMesh`) "MuzzleFlashSocket"))))
    (else
      ;[1 1 1] This is AI
      (return (`Pawn.GetBaseAimRotation` (`self.OwningPawn`))))))

(fn `UserConstructionScript`)