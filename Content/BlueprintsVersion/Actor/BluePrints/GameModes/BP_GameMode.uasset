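; Game mode that decides win or loss for a level by tracking enemy and player deaths.
; On BeginPlay it counts all BP_BaseAI actors, binds to their destruction and the player's death, and pre-creates a results widget.
; Destroying the last enemy shows the win screen, notifies the player and loads the main menu through BP_ENDGameInstance after a delay.
; Player death shows the lose screen with cursor and UI-only input.
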(event `self.ReceiveBeginPlay`
  (bind _outactors (`GameplayStatics.GetAllActorsOfClass` "/Game/BlueprintsVersion/Actor/BluePrints/BP_BaseAI.BP_BaseAI_C"))
  (set `self.NumberOfEnemies` (`KismetArrayLibrary.Array_Length` _outactors))
  (for _array_element _outactors
    (add `self.OnDestroyed` _array_element (delegate `EnemyDestroyed`)))
  (bind _returnvalue (`GameplayStatics.GetActorOfClass` "/Game/BlueprintsVersion/Actor/BluePrints/BP_Player.BP_Player_C"))
  (bind _output_get (set `self.ActivePlayer` _returnvalue))
  (add `/Game/BlueprintsVersion/Actor/BluePrints/BP_Player.OnDeathFinished` _output_get (`|CreateDelegate` :!event `PlayerDestroyed`))
  (bind _returnvalue_2 (`GameplayStatics.GetActorOfClass` (`self.PlayerControllerClass`)))
  (bind _output_get_2 (set `self.ActivePC` _returnvalue_2))
  (bind _returnvalue_3 (`|CreateWidget` (`self.ResultsClass`) _output_get_2))
  (set `self.ResultsWidget` _returnvalue_3)
  (bind _asbp_endgame_instance (cast `/Game/Core/GameInstance/BP_ENDGameInstance` (`GameplayStatics.GetGameInstance`))
    (:`then`
      (set `self.GameInstanceEnd` _asbp_endgame_instance))
    (:`CastFailed`
      (`KismetSystemLibrary.PrintString` "Wrong Game Instance"))))

(event `EnemyDestroyed` :!signature `self.OnDestroyed`
  (params (DestroyedActor :type "Actor Object Reference"))
  (bind _resultswidget (`self.ResultsWidget`))
  ;[1 1 1] Coded
  (bind _result (`/Engine/EditorBlueprintResources/StandardMacros.DecrementInt` (`self.NumberOfEnemies`))
    (:`  `
      (if (== _result 0)
        (`/Game/Core/Widgets/WBP_ResultsScreen.SetWin` _resultswidget)
        (`UserWidget.AddToViewport` _resultswidget 0)
        (`KismetSystemLibrary.K2_SetTimerDelegate` (delegate `LoadMainMenu`) (`self.TimeToSeeWinScreen`))
        (`/Game/BlueprintsVersion/Actor/BluePrints/BP_Player.WonLevel` (`self.ActivePlayer`))))))

(event `LoadMainMenu`
  ;[1 1 1] Coded
  (`/Game/Core/GameInstance/BP_ENDGameInstance.LoadMainMenu` (`self.GameInstanceEnd`)))

(event `PlayerDestroyed`
  (bind _resultswidget (`self.ResultsWidget`))
  (bind _activepc (`self.ActivePC`))
  ;[1 1 1] Coded
  (`/Game/Core/Widgets/WBP_ResultsScreen.SetLose` _resultswidget)
  (set `PlayerController.bShowMouseCursor` true _activepc)
  (`WidgetBlueprintLibrary.SetInputMode_UIOnlyEx` _activepc null "LockAlways")
  (`UserWidget.AddToViewport` _resultswidget 0))

(fn `UserConstructionScript`)