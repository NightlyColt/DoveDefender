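; Base projectile actor that damages whatever overlaps its collision component, then destroys itself.
; The overlap applies the configurable damage to the other actor, crediting the instigator's controller and passing the instigator as damage causer.
; A one-shot timer set on BeginPlay limits its lifetime, and the construction script sets the collision's world scale from a projectile scale variable.
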(event `self.Collision.OnComponentBeginOverlap`
  (params (OverlappedComponent :type "PrimitiveComponent Object Reference") (OtherActor :type "Actor Object Reference") (OtherComp :type "PrimitiveComponent Object Reference") (OtherBodyIndex :type Integer) (bFromSweep :type Boolean) (SweepResult :type "HitResult Structure (by ref)"))
  ;[1 1 1] Coded
  (`GameplayStatics.ApplyDamage` OtherActor (`self.Damage`) (`self.GetInstigatorController`) (`self.GetInstigator`))
  (`self.K2_DestroyActor`))

(event `self.ReceiveBeginPlay`
  ;[1 1 1] Coded
  (bind _returnvalue (`KismetSystemLibrary.K2_SetTimerDelegate` (`|CreateDelegate` :!event `TimerEnded`) (`self.TimeToDestroy`)))
  (set `self.DestroyTimerHandle` _returnvalue))

(event `TimerEnded`
  ;[1 1 1] Coded
  (`self.K2_DestroyActor`))

(fn `UserConstructionScript`
  (`SceneComponent.SetWorldScale3D` (`self.Collision`) (`self.ProjectileScale`)))