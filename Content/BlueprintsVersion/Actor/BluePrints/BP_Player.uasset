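; BP_Player is the player-controlled character, extending a parent character class with input handling, a HUD and level-end behaviour.
; Axis inputs drive control-yaw-relative movement and camera look, while Shoot and Reload actions forward to character functions.
; BeginPlay creates the HUD and reloads the weapon; overridden health and ammo events update that HUD.
; Death and winning disable input and remove the HUD, and health pickup is allowed only below full health.
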(event `self.ReceiveBeginPlay`
  ;[1 1 1] Coded
  (`parent.ReceiveBeginPlay`)
  (bind _asplayer_controller (cast `PlayerController` (`self.GetController`))
    (:`then`
      (bind _output_get (set `self.PlayerController` _asplayer_controller))
      (bind _returnvalue (`|CreateWidget` "/Game/Core/Widgets/WBP_HUD.WBP_HUD_C" _output_get))
      (bind _output_get_2 (set `self.HUD` _returnvalue))
      (`UserWidget.AddToViewport` _output_get_2 0)
      (`/Game/BlueprintsVersion/Actor/BluePrints/BP_BaseWeapon.Reload` (`self.CurrentWeapon`)))
    (:`CastFailed`
      (`KismetSystemLibrary.PrintString` "Need Player for HUD"))))

(event `InputAxis|TurnTo`
  (params (AxisValue :type "Float (single-precision)"))
  ;[1 1 1] Coded
  ;;[1 1 1] Rotation
  (`self.AddControllerYawInput` AxisValue))

(event `InputAxis|LookUp`
  (params (AxisValue :type "Float (single-precision)"))
  ;[1 1 1] Coded
  ;;[1 1 1] Rotation
  (`self.AddControllerPitchInput` AxisValue))

(event `InputAxis|MoveForward`
  (params (AxisValue :type "Float (single-precision)"))
  (bind (_returnvalue_roll _returnvalue_pitch _returnvalue_yaw) (`KismetMathLibrary.BreakRotator` (`self.GetControlRotation`)))
  ;[1 1 1] Coded
  (`self.AddMovementInput` (`KismetMathLibrary.GetForwardVector` (`KismetMathLibrary.MakeRotator` 0.0 0.0 _returnvalue_yaw)) AxisValue))

(event `self.CharacterDeath`
  (params (Ratio :type "Float (single-precision)"))
  ;[1 1 1] Coded
  (`self.DisableInput` self (`self.PlayerController`))
  (`parent.CharacterDeath` 0.0)
  (`Widget.RemoveFromParent` (`self.HUD`)))

(event `InputAxis|MoveSideways`
  (params (AxisValue :type "Float (single-precision)"))
  (bind (_returnvalue_roll _returnvalue_pitch _returnvalue_yaw) (`KismetMathLibrary.BreakRotator` (`self.GetControlRotation`)))
  ;[1 1 1] Coded
  (`self.AddMovementInput` (`KismetMathLibrary.GetRightVector` (`KismetMathLibrary.MakeRotator` 0.0 0.0 _returnvalue_yaw)) AxisValue))

(event `self.CharacterDamaged`
  (params (Ratio :type "Float (single-precision)"))
  ;[1 1 1] Coded
  (`parent.CharacterDamaged` 0.0)
  (`/Game/Core/Widgets/WBP_HUD.SetHealth` (`self.HUD`) Ratio))

(event `InputAction|Shoot`
  (params (Key :type "Key Structure"))
  ;[1 1 1] Coded
  (:`Pressed`
    (`self.CharacterShoot`)))

(event `InputAction|Reload`
  (params (Key :type "Key Structure"))
  ;[1 1 1] Coded
  (:`Pressed`
    (`self.CharacterReload`)))

(event `self.CharacterDeathFinished`
  ;[1 1 1] Coded
  (`parent.CharacterDeathFinished`)
  (`self.OnDeathFinished`))

(event `WonLevel`
  ;[1 1 1] Coded
  (`self.DisableInput` self (`self.PlayerController`))
  (`Widget.RemoveFromParent` (`self.HUD`))
  (`MovementComponent.StopMovementImmediately` (`self.CharacterMovement`))
  (`PrimitiveComponent.SetCollisionEnabled` (`self.CapsuleComponent`) "NoCollision"))

(event `self.CurrentAmmoChanged`
  (params (Current :type "Float (single-precision)") (Max :type "Float (single-precision)"))
  ;[1 1 1] Coded
  (`parent.CurrentAmmoChanged` Current Max)
  (`MyUserWidget.SetAmmo` (`self.HUD`) Current Max))

(event `self.CharacterHeal`
  (params (Ratio :type "Float (single-precision)"))
  (`parent.CharacterHeal` Ratio)
  (`MyUserWidget.SetHealth` (`self.HUD`) Ratio))

(fn `CanPickupHealth`
  (returns (Yes :type Boolean))
  (return (not (`HealthComponent.IsFullHealth` (`self.BP_Health_Component`)))))

(fn `UserConstructionScript`
  (`parent.UserConstructionScript`))