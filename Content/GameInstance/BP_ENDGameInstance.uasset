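; BP_ENDGameInstance is a Game Instance that handles level switching and quitting the game.
; Events load the first level, reload the current one or open the main menu at index 0 of the Levels array.
; All three route through LoadLevelSafe, which validates the index, stores it as CurrentLevelIndex and opens that level by name, printing an error for invalid indices.
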(event `LoadFirstLevel`
  (`self.LoadLevelSafe` (`self.FirstLevelIndex`)))

(event `QuitEvent`
  (`KismetSystemLibrary.QuitGame` null "Quit"))

(event `LoadMainMenu`
  (`self.LoadLevelSafe` 0))

(event `ReloadLevel`
  (`self.LoadLevelSafe` (`self.CurrentLevelIndex`)))

(fn `LoadLevelSafe`
  (params (Index :type Integer))
  (if (`KismetArrayLibrary.Array_IsValidIndex` (`self.Levels`) Index)
    (set `self.CurrentLevelIndex` Index)
    (`GameplayStatics.OpenLevel` (`|GetArrayItem` (`self.Levels`) (`self.CurrentLevelIndex`)))
    (else
      (`KismetSystemLibrary.PrintString` (`KismetStringLibrary.Concat_StrStr` "Invalid Index: " (`KismetStringLibrary.Conv_IntToString` Index))))))